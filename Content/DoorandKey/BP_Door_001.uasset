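; BP_Door_001 is a key-locked door that moves the first-person player on to the next level area.
; When something overlaps its Box while HasKey is true, it casts to BP_FirstPersonCharacter and teleports it to DestLocation with a fixed rotation.
; It then rebuilds the character's widgets, sets Ammo to NextLevelAmmo and starts the toxic gas actor held in Gas1Ref.
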(event `self.Box.OnComponentBeginOverlap`
  (params (OverlappedComponent :type "PrimitiveComponent Object Reference") (OtherActor :type "Actor Object Reference") (OtherComp :type "PrimitiveComponent Object Reference") (OtherBodyIndex :type Integer) (bFromSweep :type Boolean) (SweepResult :type "HitResult Structure (by ref)"))
  (if (`self.Has Key?`)
    (`|ExecutionSequence`
      (:`then_0`
        (bind _asbp_first_person_character (cast `/Game/FirstPerson/Blueprints/BP_FirstPersonCharacter` OtherActor))
        (`self.K2_TeleportTo` _asbp_first_person_character (`self.Dest Location`) (struct :`Yaw` -180.0))
        (`WidgetLayoutLibrary.RemoveAllWidgets`)
        (`/Game/FirstPerson/Blueprints/BP_FirstPersonCharacter.Initialize widgets` _asbp_first_person_character)
        (set `/Game/FirstPerson/Blueprints/BP_FirstPersonCharacter.Ammo` (`self.NextLevelAmmo`) _asbp_first_person_character)
        (bind _asbp_toxic_gas_1 (cast `/Game/assets/Blueprints/BP_ToxicGas1` (`self.gas1 ref`)))
        (`/Game/assets/Blueprints/BP_ToxicGas1.start gas` _asbp_toxic_gas_1)))))

(fn `UserConstructionScript`)