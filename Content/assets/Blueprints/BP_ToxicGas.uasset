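; BP_ToxicGas is a gas hazard that turns dangerous after a safety delay.
; On BeginPlay, a Timeline moves its local height fog while delays of SafetyTime run in parallel.
; When they end, it flags the gas as high, shows a warning widget and starts a looping timer.
; Each timer tick applies radial damage around the actor, ignoring the big and small enemy references.
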(event `self.ReceiveBeginPlay`
  (`|ExecutionSequence`
    (:`then_0`
      (bind (_direction _newtrack_0) (`Timeline|Move`)
        (:`Update`
          (`SceneComponent.K2_SetRelativeLocation` (`self.LocalHeightFog`) _newtrack_0 false false))))
    (:`then_1`
      (`KismetSystemLibrary.Delay` (`self.SafetyTime`))
      (`KismetSystemLibrary.PrintString` "Gas Levels critical")
      (set `self.IsGasLevelHigh?` true)
      (`self.warning text`))
    (:`then_2`
      (`KismetSystemLibrary.Delay` (`self.SafetyTime`))
      (`KismetSystemLibrary.K2_SetTimerDelegate` (delegate `tick damage`) (`self.TickTime`) true))))

(event `warning text`
  (if (`self.IsGasLevelHigh?`)
    (bind _returnvalue (`|CreateWidget` "/Game/UI/WB_Warning.WB_Warning_C"))
    (bind _output_get (set `self.Warning widget` _returnvalue))
    (`UserWidget.AddToViewport` _output_get 0)))

(event `tick damage`
  (`GameplayStatics.ApplyRadialDamage` (`self.Base Damage`) (`self.K2_GetActorLocation`) (`self.Damage Radius`) null (`|MakeArray` (`self.EnemyBig Ref`) (`self.EnemySmall Ref`) :!type "Actor Object Reference") null null))

(fn `UserConstructionScript`)